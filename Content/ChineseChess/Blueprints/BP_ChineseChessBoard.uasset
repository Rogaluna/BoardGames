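; Chinese chess (Xiangqi) board actor that seats players as Chu or Han and relays their slot clicks during a match.
; Board and slot clicks go through the local PlayerController as remote event messages, with slot positions packed as JSON.
; RemoteCall either assigns a new player the open camp, random if both are free, or resolves the slot and handles its click.
; Entering activates that camp's camera and blends the view to the board; leaving restores the pawn view.
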(event Custom|Execute_PlayerEntered
  (params (PlayerCamp :type EChineseChessPlayer%20Enum :default "Chu") (Player :type Player%20State%20Object%20Reference))
  (bind _camera_chu (Variables|Default|GetCamera_Chu))
  (bind _camera_han (Variables|Default|GetCamera_Han))
  (switch Utilities|FlowControl|Switch|SwitchonEChineseChessPlayer PlayerCamp
    (:Chu
      (Components|Activation|Deactivate _camera_han)
      (Components|Activation|Activate _camera_chu true))
    (:Han
      (Components|Activation|Deactivate _camera_chu)
      (Components|Activation|Activate _camera_han true)))
  (Game|Player|SetViewTargetwithBlend (Game|GetPlayerController 0) self 0.0 "VTBlend_Linear" 0.0 false))

(event Custom|Execute_PlayerLeft
  (params (PlayerCamp :type EChineseChessPlayer%20Enum :default "Chu") (Player :type Player%20State%20Object%20Reference))
  (bind _returnvalue (Game|GetPlayerController 0))
  (Utilities|IsValid _returnvalue
    (:Is%20Valid
      (Game|Player|SetViewTargetwithBlend _returnvalue (Game|Player|GetPlayerPawn 0) 0.0 "VTBlend_Linear" 0.0 false))))

(event Custom|Execute_SlotClicked
  (params (Slot :type Chinese%20Chess%20Board%20Slot%20Object%20Reference))
  (if (Class|ChineseChessManager|GetIsGameing (Class|ChineseChessBoard|GetGameManager))
    (Class|RemoteCallableControllerInterface|RemoteEvent(Message) (Game|GetPlayerController 0) self (Utilities|Struct|MakeRemoteCallableData (Variables|/Script/Engine.Controller|GetPlayerState (Game|GetPlayerController 0)) (Class|RomoteCallableBlueprintFunctionLibrary|CreateJsonString "Slot" (Utilities|String|ToString(Vector2d) (Class|ChineseChessBoardSlot|GetSlotPos Slot)))))))

(event MouseInput|EventActorOnClicked
  (params (ButtonPressed :type Key%20Structure))
  (bind _returnvalue (Game|GetPlayerController 0))
  (Class|RemoteCallableControllerInterface|RemoteEvent(Message) _returnvalue self (Utilities|Struct|MakeRemoteCallableData (Variables|/Script/Engine.Controller|GetPlayerState _returnvalue))))

(event EventBeginPlay
  (EventDispatchers|AssignSlotClicked (delegate Custom|Execute_SlotClicked)))

(event EventRemoteCall
  (params (RCData :type Remote%20Callable%20Data%20Structure))
  (bind (_ps _data) (Utilities|Struct|BreakRemoteCallableData RCData))
  (bind _returnvalue (Class|ChineseChessBoard|GetGameManager))
  (bind (_outvalue _returnvalue_2) (Class|RomoteCallableBlueprintFunctionLibrary|ParseJsonString _data "Slot"))
  (if (Class|RyRuntimeStringHelpers|IsEmpty _data)
    (if (not (Class|ChineseChessManager|IsEntered _returnvalue _ps))
      (bind _outawaitstate (Class|ChineseChessManager|WaitPlayer _returnvalue))
      (switch Utilities|FlowControl|Switch|SwitchonEChineseChessAwaitState _outawaitstate
        (:Wait_Chu
          (Class|ChineseChessManager|OnPlayerEntered _returnvalue "Chu" _ps :!label _label))
        (:Wait_Han
          (Class|ChineseChessManager|OnPlayerEntered _returnvalue "Han" _ps :!label _label_2))
        (:Wait_BothSides
          (if (Math|Random|RandomBool)
            (goto _label)
            (else
              (goto _label_2))))))
    (else
      (Utilities|FlowControl|Sequence
        (:then_0
          (if _returnvalue_2
            (bind _returnvalue_3 (Class|ChineseChessBoard|GetSlot (Class|RomoteCallableBlueprintFunctionLibrary|DataConvertVector2D _outvalue)))
            (Class|ChineseChessBoard|HandleSlotClicked _returnvalue_3 _ps)))))))

(fn ConstructionScript)