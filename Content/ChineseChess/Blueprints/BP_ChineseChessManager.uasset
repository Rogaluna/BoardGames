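; Manager for a networked Chinese chess match between Chu and Han, handling seating, game start/end, checks, surrender and camp switching.
; Game-action delegates fan out to multicasts that drive the menu, log and tip widgets, with camp switches rotating board and pieces and swapping cameras.
; Local menu requests reach game logic as string payloads through PlayerController RemoteEventMessage.
; An external AI process hook sends the feature map and only prints replies.
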(event Custom|Mulitcast_On%20Player%20Entered
  (params (PlayerState :type Player%20State%20Object%20Reference) (Type :type EChineseChessPlayer%20Enum :default "Chu"))
  (bind _returnvalue (Game|GetPlayerController PlayerState))
  (bind _returnvalue_2 (Utilities|String|EnumtoString Type))
  (bind _returnvalue_3 (Utilities|String|Append _returnvalue_2 "已入座"))
  (Utilities|IsValid (Variables|Default|GetGame%20Menu)
    (:Is%20Valid
      (bind _returnvalue_4 (UserInterface|CreateWidget (Variables|Default|GetTipsWidgetClass) (Game|GetPlayerController 0) :!label _label))
      (bind _asuw_tips (Utilities|Casting|CastToUW_Tips _returnvalue_4))
      (Variables|/BoardGames/ChineseChess/Blueprints/UI/UW_Tips.UW_Tips_C|SetDisplayText _asuw_tips (Utilities|Text|ToText(String) _returnvalue_3))
      (UserInterface|Viewport|AddtoViewport _asuw_tips 0)
      (CallFunction|PrintLog _returnvalue_3 "(R=0.000000,G=0.023484,B=1.000000,A=1.000000)"))
    (:Is%20Not%20Valid
      (Utilities|IsValid _returnvalue
        (:Is%20Valid
          (if (Pawn|IsLocalPlayerController _returnvalue)
            (Utilities|FlowControl|Sequence
              (:then_0
                (bind _returnvalue_5 (UserInterface|CreateWidget (Variables|Default|GetMenuWidgetClass) _returnvalue))
                (bind _asuw_game_menu (Utilities|Casting|CastToUW_GameMenu _returnvalue_5))
                (Variables|Default|SetGame%20Menu _asuw_game_menu)
                (Variables|/BoardGames/ChineseChess/Blueprints/UI/UW_GameMenu.UW_GameMenu_C|SetGameManager _asuw_game_menu self)
                (Default|UpdateGameStartBtnStyle _asuw_game_menu)
                (UserInterface|Viewport|AddtoViewport _asuw_game_menu 0)
                (bind _asbp_chinese_chess_board (Utilities|Casting|CastToBP_ChineseChessBoard (Class|BoardGameManager|GetBoard)))
                (Default|ExecutePlayerEntered _asbp_chinese_chess_board Type PlayerState))
              (:then_1
                (goto _label)))))))))

(event Custom|Local_StartGame
  (bind _returnvalue (Game|GetPlayerController 0))
  (Class|RemoteCallableControllerInterface|RemoteEvent(Message) _returnvalue self (Utilities|Struct|MakeRemoteCallableData (Variables|/Script/Engine.Controller|GetPlayerState _returnvalue) "StartGame")))

(event Custom|Multicast_OnSwitchCamp
  (bind _asbp_chinese_chess_board (Utilities|Casting|CastToBP_ChineseChessBoard (Class|BoardGameManager|GetBoard)))
  (if (Components|Activation|IsActive (Variables|/BoardGames/ChineseChess/Blueprints/BP_ChineseChessBoard.BP_ChineseChessBoard_C|GetCamera_Chu _asbp_chinese_chess_board))
    (Components|Activation|Deactivate (Variables|/BoardGames/ChineseChess/Blueprints/BP_ChineseChessBoard.BP_ChineseChessBoard_C|GetCamera_Chu _asbp_chinese_chess_board))
    (Components|Activation|Activate (Variables|/BoardGames/ChineseChess/Blueprints/BP_ChineseChessBoard.BP_ChineseChessBoard_C|GetCamera_Han _asbp_chinese_chess_board) false)
    (else
      (Components|Activation|Deactivate (Variables|/BoardGames/ChineseChess/Blueprints/BP_ChineseChessBoard.BP_ChineseChessBoard_C|GetCamera_Han _asbp_chinese_chess_board))
      (Components|Activation|Activate (Variables|/BoardGames/ChineseChess/Blueprints/BP_ChineseChessBoard.BP_ChineseChessBoard_C|GetCamera_Chu _asbp_chinese_chess_board) false))))

(event Custom|StartAIProcess
  (bind _returnvalue (Class|RuntimeProcessBlueprintFunctionLibrary|CreateProcessManager 9513 false "Z:/XediaDocument/Project/Python/ue-connection/dist/helloworld.exe"))
  (Variables|Default|SetAIProcess _returnvalue)
  (Utilities|FlowControl|Sequence
    (:then_0
      (EventDispatchers|BindEventtoOnProcessConnected (Variables|Default|GetAIProcess) (delegate Custom|AIConnected)))
    (:then_1
      (EventDispatchers|BindEventtoOnMessageReceived (Variables|Default|GetAIProcess) (delegate Custom|MessageReceived)))))

(event Custom|Multicast_Check
  (params (PlayerState :type Player%20State%20Object%20Reference))
  (bind _returnvalue (Game|GetPlayerController 0))
  (Utilities|IsValid _returnvalue
    (:Is%20Valid
      (bind (_playercamp _returnvalue_2) (Class|ChineseChessManager|GetPlayerCamp PlayerState))
      (if _returnvalue_2
        (bind _returnvalue_3 (UserInterface|CreateWidget (Variables|Default|GetTipsWidgetClass) _returnvalue))
        (bind _asuw_tips (Utilities|Casting|CastToUW_Tips _returnvalue_3))
        (switch Utilities|FlowControl|Switch|SwitchonEChineseChessPlayer _playercamp
          (:Chu
            (Variables|/BoardGames/ChineseChess/Blueprints/UI/UW_Tips.UW_Tips_C|SetDisplayText _asuw_tips "楚 将军"))
          (:Han
            (Variables|/BoardGames/ChineseChess/Blueprints/UI/UW_Tips.UW_Tips_C|SetDisplayText _asuw_tips "汉 将军")))
        (UserInterface|Viewport|AddtoViewport _asuw_tips 0)))))

(event Custom|Multicast_CheckMate
  (params (PlayerState :type Player%20State%20Object%20Reference))
  (bind _returnvalue (Game|GetPlayerController 0))
  (Utilities|IsValid _returnvalue
    (:Is%20Valid
      (bind (_playercamp _returnvalue_2) (Class|ChineseChessManager|GetPlayerCamp PlayerState))
      (if _returnvalue_2
        (bind _returnvalue_3 (UserInterface|CreateWidget (Variables|Default|GetTipsWidgetClass) _returnvalue))
        (bind _asuw_tips (Utilities|Casting|CastToUW_Tips _returnvalue_3))
        (switch Utilities|FlowControl|Switch|SwitchonEChineseChessPlayer _playercamp
          (:Chu
            (Variables|/BoardGames/ChineseChess/Blueprints/UI/UW_Tips.UW_Tips_C|SetDisplayText _asuw_tips "楚 获胜"))
          (:Han
            (Variables|/BoardGames/ChineseChess/Blueprints/UI/UW_Tips.UW_Tips_C|SetDisplayText _asuw_tips "汉 获胜")))
        (UserInterface|Viewport|AddtoViewport _asuw_tips 0)))))

(event Custom|Multicast_SwitchRound
  (params (PlayerState :type Player%20State%20Object%20Reference))
  (Utilities|IsValid (Game|GetPlayerController 0)
    (:Is%20Valid
      (bind (_playercamp _returnvalue) (Class|ChineseChessManager|GetPlayerCamp PlayerState))
      (if _returnvalue
        (bind _returnvalue_2 (UserInterface|CreateWidget (Variables|Default|GetTipsWidgetClass)))
        (bind _asuw_tips (Utilities|Casting|CastToUW_Tips _returnvalue_2))
        (switch Utilities|FlowControl|Switch|SwitchonEChineseChessPlayer _playercamp
          (:Chu
            (Variables|/BoardGames/ChineseChess/Blueprints/UI/UW_Tips.UW_Tips_C|SetDisplayText _asuw_tips "楚军回合"))
          (:Han
            (Variables|/BoardGames/ChineseChess/Blueprints/UI/UW_Tips.UW_Tips_C|SetDisplayText _asuw_tips "汉军回合")))
        (UserInterface|Viewport|AddtoViewport _asuw_tips 0)))))

(event Custom|AIConnected
  (bind _returnvalue (Class|ChineseChessManager|GetFeatureMap))
  (Class|RuntimeProcessManager|SendMessagetoClientByte (Variables|Default|GetAIProcess) _returnvalue))

(event Custom|MessageReceived
  (params (Message :type String))
  (Development|PrintString Message true true "(R=1.000000,G=0.000000,B=0.010551,A=1.000000)" 2e+04))

(event Custom|Execute_PlayerEntered
  (params (PlayerCamp :type EChineseChessPlayer%20Enum :default "Chu") (Player :type Player%20State%20Object%20Reference))
  (CallFunction|MulitcastonPlayerEntered Player PlayerCamp))

(event Custom|Execute_GameAction
  (params (GameState :type EChineseChessGameState%20Enum :default "None") (Player :type Player%20State%20Object%20Reference))
  (switch Utilities|FlowControl|Switch|SwitchonEChineseChessGameState GameState
    (:GameStart
      (CallFunction|MulticastonGameStart))
    (:GameOver
      (CallFunction|MulticastonGameOver))
    (:IllegalMove
      (CallFunction|MulticastIllegalMove Player))
    (:Check
      (CallFunction|MulticastCheck Player))
    (:CheckMate
      (CallFunction|MulticastCheckMate Player))
    (:GiveUp
      (CallFunction|MulticastGiveUp Player))
    (:RoundSwitch
      (CallFunction|MulticastSwitchRound Player))
    (:CampSwitch
      (bind _asbp_chinese_chess_board (Utilities|Casting|CastToBP_ChineseChessBoard (Class|BoardGameManager|GetBoard)))
      (bind _returnvalue (Transformation|SetActorRotation _asbp_chinese_chess_board (Math|Rotator|MakeRotator (.Roll (Math|Rotator|BreakRotator (Transformation|GetActorRotation _asbp_chinese_chess_board))) (.Pitch (Math|Rotator|BreakRotator (Transformation|GetActorRotation _asbp_chinese_chess_board))) (Math|Float|%(Float) (+ (.Yaw (Math|Rotator|BreakRotator (Transformation|GetActorRotation _asbp_chinese_chess_board))) 1.8e+02) 3.6e+02))))
      (if _returnvalue
        (for _array_element (Class|ChineseChessManager|GetPawnArray)
          (Transformation|SetActorLocationAndRotation _array_element (Transformation|GetWorldLocation (Class|ChineseChessPawn|GetSlot _array_element)) (Math|Rotator|MakeRotator (.Roll (Math|Rotator|BreakRotator (Transformation|GetActorRotation _array_element))) (.Pitch (Math|Rotator|BreakRotator (Transformation|GetActorRotation _array_element))) (Math|Float|%(Float) (+ (.Yaw (Math|Rotator|BreakRotator (Transformation|GetActorRotation _array_element))) 1.8e+02) 3.6e+02))))
        (CallFunction|MulticastonSwitchCamp)))))

(event Custom|Execute_PlayerLeft
  (params (PlayerCamp :type EChineseChessPlayer%20Enum :default "Chu") (Player :type Player%20State%20Object%20Reference))
  (CallFunction|MulticastonPlayerLeft Player PlayerCamp))

(event Custom|Multicast_OnGameStart
  (bind _game_menu (Variables|Default|GetGame%20Menu))
  (Utilities|IsValid _game_menu
    (:Is%20Valid
      (Default|OnStartGame _game_menu)
      (bind _returnvalue (UserInterface|CreateWidget (Variables|Default|GetTipsWidgetClass) (Game|GetPlayerController 0)))
      (bind _asuw_tips (Utilities|Casting|CastToUW_Tips _returnvalue))
      (Variables|/BoardGames/ChineseChess/Blueprints/UI/UW_Tips.UW_Tips_C|SetDisplayText _asuw_tips "游戏开始")
      (UserInterface|Viewport|AddtoViewport _asuw_tips 0)
      (CallFunction|PrintLog "游戏开始" "(R=0.033466,G=1.000000,B=0.000000,A=1.000000)"))))

(event Custom|Multicast_OnGameOver
  (bind _game_menu (Variables|Default|GetGame%20Menu))
  (Utilities|IsValid _game_menu
    (:Is%20Valid
      (Default|OnStartGame _game_menu)
      (bind _returnvalue (UserInterface|CreateWidget (Variables|Default|GetTipsWidgetClass) (Game|GetPlayerController 0)))
      (bind _asuw_tips (Utilities|Casting|CastToUW_Tips _returnvalue))
      (Variables|/BoardGames/ChineseChess/Blueprints/UI/UW_Tips.UW_Tips_C|SetDisplayText _asuw_tips "游戏结束")
      (UserInterface|Viewport|AddtoViewport _asuw_tips 0)
      (CallFunction|PrintLog "游戏结束" "(R=1.000000,G=0.861242,B=0.000000,A=1.000000)"))))

(event Custom|Local_GiveUp
  (bind _returnvalue (Game|GetPlayerController 0))
  (Class|RemoteCallableControllerInterface|RemoteEvent(Message) _returnvalue self (Utilities|Struct|MakeRemoteCallableData (Variables|/Script/Engine.Controller|GetPlayerState _returnvalue) "GiveUp")))

(event Custom|Local_Leave
  (bind _returnvalue (Game|GetPlayerController 0))
  (Class|RemoteCallableControllerInterface|RemoteEvent(Message) _returnvalue self (Utilities|Struct|MakeRemoteCallableData (Variables|/Script/Engine.Controller|GetPlayerState _returnvalue) "Leave"))
  (Widget|RemovefromParent (Variables|Default|GetGame%20Menu))
  (Variables|Default|SetGame%20Menu 0))

(event Custom|Multicast_GiveUp
  (params (PlayerState :type Player%20State%20Object%20Reference))
  (bind _returnvalue (Game|GetPlayerController 0))
  (Utilities|IsValid _returnvalue
    (:Is%20Valid
      (bind (_playercamp _returnvalue_2) (Class|ChineseChessManager|GetPlayerCamp PlayerState))
      (if _returnvalue_2
        (bind _returnvalue_3 (UserInterface|CreateWidget (Variables|Default|GetTipsWidgetClass) _returnvalue))
        (bind _asuw_tips (Utilities|Casting|CastToUW_Tips _returnvalue_3))
        (switch Utilities|FlowControl|Switch|SwitchonEChineseChessPlayer _playercamp
          (:Chu
            (bind _output_get (Variables|/BoardGames/ChineseChess/Blueprints/UI/UW_Tips.UW_Tips_C|SetDisplayText _asuw_tips "楚 认输"))
            (CallFunction|PrintLog (Utilities|String|ToString(Text) _output_get) "(R=1.000000,G=0.000000,B=0.777960,A=1.000000)"))
          (:Han
            (bind _output_get_2 (Variables|/BoardGames/ChineseChess/Blueprints/UI/UW_Tips.UW_Tips_C|SetDisplayText _asuw_tips "汉 认输"))
            (CallFunction|PrintLog (Utilities|String|ToString(Text) _output_get_2) "(R=1.000000,G=0.000000,B=0.777960,A=1.000000)")))
        (UserInterface|Viewport|AddtoViewport _asuw_tips 0)
        (Default|OnGiveUp (Variables|Default|GetGame%20Menu))))))

(event Custom|Multicast_IllegalMove
  (params (PlayerState :type Player%20State%20Object%20Reference))
  (bind _returnvalue (Game|GetPlayerController PlayerState))
  (bind _returnvalue_2 (Game|GetPlayerController 0))
  (Utilities|IsValid _returnvalue_2
    (:Is%20Valid
      (if (== _returnvalue _returnvalue_2)
        (bind _returnvalue_3 (UserInterface|CreateWidget (Variables|Default|GetTipsWidgetClass) _returnvalue))
        (bind _asuw_tips (Utilities|Casting|CastToUW_Tips _returnvalue_3))
        (Variables|/BoardGames/ChineseChess/Blueprints/UI/UW_Tips.UW_Tips_C|SetDisplayText _asuw_tips "请先解将")
        (UserInterface|Viewport|AddtoViewport _asuw_tips 0)))))

(event Custom|Print%20Log
  (params (LogString :type String) (LogColor :type Linear%20Color%20Structure))
  (Utilities|IsValid (Variables|Default|GetGame%20Menu)
    (:Is%20Valid
      (Default|OnPrintLog (Variables|Default|GetGame%20Menu) LogString LogColor))))

(event Custom|Local%20Switch%20Camp
  (params (Type :type EChineseChessPlayer%20Enum :default "Chu"))
  (bind _returnvalue (Game|GetPlayerController 0))
  (Class|RemoteCallableControllerInterface|RemoteEvent(Message) _returnvalue self (Utilities|Struct|MakeRemoteCallableData (Variables|/Script/Engine.Controller|GetPlayerState _returnvalue) (Utilities|Select :Index Type :Chu "SwitchCamp_Chu" :Han "SwitchCamp_Han"))))

(event Custom|Multicast_On%20Player%20Left
  (params (PlayerState :type Player%20State%20Object%20Reference) (Type :type EChineseChessPlayer%20Enum :default "Chu"))
  (bind _returnvalue (Utilities|String|EnumtoString Type))
  (bind _returnvalue_2 (Utilities|String|Append _returnvalue "已离开"))
  (Utilities|IsValid (Variables|Default|GetGame%20Menu)
    (:Is%20Valid
      (bind _returnvalue_3 (UserInterface|CreateWidget (Variables|Default|GetTipsWidgetClass) (Game|GetPlayerController 0)))
      (bind _asuw_tips (Utilities|Casting|CastToUW_Tips _returnvalue_3))
      (Variables|/BoardGames/ChineseChess/Blueprints/UI/UW_Tips.UW_Tips_C|SetDisplayText _asuw_tips (Utilities|Text|ToText(String) _returnvalue_2))
      (UserInterface|Viewport|AddtoViewport _asuw_tips 0)
      (CallFunction|PrintLog _returnvalue_2 "(R=0.000000,G=0.023484,B=1.000000,A=1.000000)"))
    (:Is%20Not%20Valid
      (if (== PlayerState (Game|GetPlayerState 0))
        (bind _asbp_chinese_chess_board (Utilities|Casting|CastToBP_ChineseChessBoard (Class|BoardGameManager|GetBoard)))
        (Default|ExecutePlayerLeft _asbp_chinese_chess_board Type)))))

(event EventNotifyPlayerChange
  (Utilities|IsValid (Variables|Default|GetGame%20Menu)
    (:Is%20Valid
      (bind _outawaitstate (Class|ChineseChessManager|WaitPlayer))
      (Default|SetSeatedPlayer (Variables|Default|GetGame%20Menu) _outawaitstate))))

(event EventBeginPlay
  (Utilities|FlowControl|Sequence
    (:then_0
      (EventDispatchers|AssignPlayerEntered (delegate Custom|Execute_PlayerEntered)))
    (:then_1
      (EventDispatchers|AssignPlayerLeft (delegate Custom|Execute_PlayerLeft)))
    (:then_2
      (EventDispatchers|AssignGameAction (delegate Custom|Execute_GameAction)))))

(event EventNotifyMovableSlotsShow
  (params (SlotPositions :type Array%20of%20Vector%202D%20Structures))
  (bind _asbp_chinese_chess_board (Utilities|Casting|CastToBP_ChineseChessBoard (Class|BoardGameManager|GetBoard)))
  (for _array_element SlotPositions
    (bind _returnvalue (Class|ChineseChessBoard|GetSlot _asbp_chinese_chess_board _array_element))
    (Class|GameBaseBoardSlot|SetColliderMaterialType _returnvalue "Default")))

(event EventNotifySlotsHide
  (bind _asbp_chinese_chess_board (Utilities|Casting|CastToBP_ChineseChessBoard (Class|BoardGameManager|GetBoard)))
  (for _array_element (Class|ChineseChessBoard|GetSlots _asbp_chinese_chess_board)
    (Class|GameBaseBoardSlot|SetColliderMaterialType _array_element "None")))

(event EventRemoteCall
  (params (RCData :type Remote%20Callable%20Data%20Structure))
  (bind (_ps _data) (Utilities|Struct|BreakRemoteCallableData RCData))
  (switch string _data
    (:StartGame
      (Class|ChineseChessManager|GameStart))
    (:GiveUp
      (Class|ChineseChessManager|GiveUp _ps))
    (:Leave
      (Class|ChineseChessManager|OnPlayerLeft _ps))
    (:SwitchCamp_Chu
      (Class|ChineseChessManager|SwitchCamp _ps "Chu"))
    (:SwitchCamp_Han
      (Class|ChineseChessManager|SwitchCamp _ps "Han"))))

(fn ConstructionScript)