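; Chinese chess cannon (Pao) pawn for the Chu side, defining which board positions it can move to or capture.
; MoveRule clears the parent's result, then steps along each direction, adding empty positions until it meets a piece.
; It then searches beyond that screen piece and adds the next occupied position only if that piece belongs to the other side.
; The event graph and construction script are empty stubs.
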(event EventBeginPlay)

(event Collision|EventActorBeginOverlap
  (params (OtherActor :type Actor%20Object%20Reference)))

(event EventTick
  (params (DeltaSeconds :type Float%20%28single-precision%29)))

(event EventPerformSelectedTeamPawn)

(event EventPerformIdlePawn)

(event EventPerformSelectedEnemyPawn)

(fn ConstructionScript)

(fn MoveRule
  (params (InBoardStatus :type Array%20of%20Bytes) (PawnPos :type Vector%202D%20Structure%20%28by%20ref%29))
  (bind _output_get (LocalVariables|SetCurrentSlotPos PawnPos))
  (bind _outpositions (|CallParentFunction InBoardStatus _output_get))
  (Utilities|FlowControl|Sequence
    (:then_0
      (Utilities|Array|Clear _outpositions))
    (:then_1
      (for _array_element (LocalVariables|GetDirections)
        (while (LocalVariables|GetbContinueInteration)
          (bind _output_get_2 (LocalVariables|SetDetectionPos (+ (Math|Conversions|ToVector2D(Vector) (* _array_element (LocalVariables|GetInterator))) (LocalVariables|GetCurrentSlotPos))))
          (if (Class|ChineseChessSetFunctionLibrary|CheckPositioninBoard _output_get_2)
            (if (!= (Utilities|Array|Get(acopy) InBoardStatus (Class|ChineseChessSetFunctionLibrary|TransformPostoIndex (LocalVariables|GetDetectionPos))) 0)
              (while (LocalVariables|GetbSearchAttackPos)
                (bind _output_get_3 (LocalVariables|SetJumpPos (+ (Math|Conversions|ToVector2D(Vector) (* _array_element (LocalVariables|GetJumpInterator))) (LocalVariables|GetDetectionPos))))
                (if (Class|ChineseChessSetFunctionLibrary|CheckPositioninBoard _output_get_3)
                  (if (!= (Utilities|Array|Get(acopy) InBoardStatus (Class|ChineseChessSetFunctionLibrary|TransformPostoIndex (LocalVariables|GetJumpPos))) 0)
                    (if (Utilities|Enum|Equal(Enum) (Class|ChineseChessSetFunctionLibrary|IsBelongto (Utilities|Array|Get(acopy) InBoardStatus (Class|ChineseChessSetFunctionLibrary|TransformPostoIndex (LocalVariables|GetJumpPos)))) (Class|ChineseChessSetFunctionLibrary|IsBelongto (Class|ChineseChessSetFunctionLibrary|Encode (Class|ChineseChessPawn|GetPawnType))))
                      _
                      (else
                        (Utilities|Array|AddUnique _outpositions (LocalVariables|GetJumpPos))))
                    (LocalVariables|SetbContinueInteration false)
                    (LocalVariables|SetbSearchAttackPos false)
                    (else
                      (Math|Integer|IncrementInt (LocalVariables|GetJumpInterator))))
                  (else
                    (LocalVariables|SetbSearchAttackPos false)
                    (LocalVariables|SetbContinueInteration false))))
              (else
                (Utilities|Array|AddUnique _outpositions (LocalVariables|GetDetectionPos))
                (Math|Integer|IncrementInt (LocalVariables|GetInterator))))
            (else
              (LocalVariables|SetbContinueInteration false))))
        (LocalVariables|SetbContinueInteration true)
        (LocalVariables|SetbSearchAttackPos true)
        (LocalVariables|SetInterator 1)
        (LocalVariables|SetJumpInterator 1)))
    (:then_2
      (return _outpositions))))