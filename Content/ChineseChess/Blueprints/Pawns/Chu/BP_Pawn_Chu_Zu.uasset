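; Chinese chess Zu (soldier) pawn Blueprint for the Chu side, with outline feedback for idle, selected ally and selected enemy states.
; MoveRule only caches the board, its size and the pawn's current slot position.
; Unconnected logic, which never runs, would derive camp-based forward steps, add sideways steps past the river, and keep in-board slots that are empty or enemy-occupied.
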(event EventBeginPlay)

(event Collision|EventActorBeginOverlap
  (params (OtherActor :type Actor%20Object%20Reference)))

(event EventTick
  (params (DeltaSeconds :type Float%20%28single-precision%29)))

(event EventPerformSelectedTeamPawn
  (Class|OutlineComponent|SetOutline (Variables|Default|GetOutline) "Blue"))

(event EventPerformIdlePawn
  (Class|OutlineComponent|SetOutline (Variables|Default|GetOutline) "None"))

(event EventPerformSelectedEnemyPawn
  (Class|OutlineComponent|SetOutline (Variables|Default|GetOutline) "Red"))

(fn ConstructionScript)

(fn MoveRule
  (Utilities|FlowControl|Sequence
    (:then_0
      (bind _aschinese_chess_board (Utilities|Casting|CastToChineseChessBoard (Class|BoardGameManager|GetBoard (Class|ChineseChessPawn|GetGameManagerPtr))))
      (LocalVariables|SetBoardPtr _aschinese_chess_board))
    (:then_1
      (LocalVariables|SetBoardSize (Class|ChineseChessBoard|GetBoardSize (LocalVariables|GetBoardPtr))))
    (:then_2
      (LocalVariables|SetCurrentSlotPos (Class|ChineseChessPawn|GetSlotPos)))))