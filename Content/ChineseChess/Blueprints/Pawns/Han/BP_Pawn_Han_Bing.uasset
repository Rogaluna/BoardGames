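; Chinese chess soldier (Bing) pawn that defines its legal moves and sets its outline for idle, team-selected and enemy-selected states.
; MoveRule clears the parent rule's result, then builds step directions from camp: one step forward, plus sideways once the pawn's Y lies across the river.
; Each target is checked against the board and kept if the slot is empty or holds an opposing-camp piece.
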(event EventBeginPlay)

(event Collision|EventActorBeginOverlap
  (params (OtherActor :type Actor%20Object%20Reference)))

(event EventTick
  (params (DeltaSeconds :type Float%20%28single-precision%29)))

(event EventPerformSelectedTeamPawn
  (Class|OutlineComponent|SetOutline (Variables|Default|GetOutline) "Blue"))

(event EventPerformIdlePawn
  (Class|OutlineComponent|SetOutline (Variables|Default|GetOutline) "None"))

(event EventPerformSelectedEnemyPawn
  (Class|OutlineComponent|SetOutline (Variables|Default|GetOutline) "Red"))

(fn ConstructionScript)

(fn MoveRule
  (params (InBoardStatus :type Array%20of%20Bytes) (PawnPos :type Vector%202D%20Structure%20%28by%20ref%29))
  (bind _y (Math|Vector2D|BreakVector2D PawnPos))
  (bind _directions (LocalVariables|GetDirections))
  (bind _directions_2 (LocalVariables|GetDirections))
  (Utilities|FlowControl|Sequence
    (:then_0
      (bind _aschinese_chess_board (Utilities|Casting|CastToChineseChessBoard (Class|BoardGameManager|GetBoard (Class|ChineseChessPawn|GetGameManagerPtr))))
      (LocalVariables|SetBoardPtr _aschinese_chess_board))
    (:then_1
      (LocalVariables|SetBoardSize (Class|ChineseChessBoard|GetBoardSize (LocalVariables|GetBoardPtr))))
    (:then_2
      (LocalVariables|SetCurrentSlotPos (Class|ChineseChessPawn|GetSlotPos))
      (bind _outpositions (|CallParentFunction InBoardStatus PawnPos))
      (Utilities|FlowControl|Sequence
        (:then_0
          (Utilities|Array|Clear _outpositions)
          (switch Utilities|FlowControl|Switch|SwitchonEChineseChessCamp (Class|ChineseChessPawn|GetCamp)
            (:Chu
              (Utilities|Array|AddUnique _directions "(X=0.000000,Y=1.000000)")
              (if (Math|Float|InRange(Float) _y 5.0 9.0)
                (Utilities|Array|AddUnique _directions_2 "(X=1.000000,Y=0.000000)" :!label _label)
                (Utilities|Array|AddUnique _directions_2 "(X=-1.000000,Y=0.000000)")))
            (:Han
              (Utilities|Array|AddUnique _directions "(X=0.000000,Y=-1.000000)")
              (if (Math|Float|InRange(Float) _y 0.0 4.0)
                (goto _label)))))
        (:then_1
          (for _array_element (LocalVariables|GetDirections)
            (bind _output_get (LocalVariables|SetDetectionPos (+ _array_element (LocalVariables|GetCurrentSlotPos))))
            (if (Class|ChineseChessBoard|CheckPositioninBoard (LocalVariables|GetBoardPtr) _output_get)
              (bind _returnvalue (Class|ChineseChessBoard|GetSlot (LocalVariables|GetBoardPtr) (LocalVariables|GetDetectionPos)))
              (if (Class|GameBaseBoardSlot|IsOccupied _returnvalue)
                (bind _aschinese_chess_pawn (Utilities|Casting|CastToChineseChessPawn (Class|GameBaseBoardSlot|GetOccupyingPawn _returnvalue)))
                (if (not (Utilities|Enum|Equal(Enum) (Class|ChineseChessPawn|GetCamp _aschinese_chess_pawn) (Class|ChineseChessPawn|GetCamp)))
                  (Utilities|Array|AddUnique _outpositions (LocalVariables|GetDetectionPos)))
                (else
                  (Utilities|Array|AddUnique _outpositions (LocalVariables|GetDetectionPos)))))))
        (:then_2
          (return _outpositions))))))