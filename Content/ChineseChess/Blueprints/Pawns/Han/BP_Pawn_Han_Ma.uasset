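; Pawn Blueprint for the Han camp's Horse (Ma) in Chinese chess, defining its legal moves and selection highlight.
; MoveRule tests each Directions offset, finding the blocking "horse leg" square by halving and truncating that offset.
; If that square is on the board and free, in-board destinations that are empty or held by the other camp are returned.
; Idle and selection events switch the outline between none, blue for team and red for enemy.
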(event EventBeginPlay)

(event Collision|EventActorBeginOverlap
  (params (OtherActor :type Actor%20Object%20Reference)))

(event EventTick
  (params (DeltaSeconds :type Float%20%28single-precision%29)))

(event EventPerformSelectedTeamPawn
  (Class|OutlineComponent|SetOutline (Variables|Default|GetOutline) "Blue"))

(event EventPerformIdlePawn
  (Class|OutlineComponent|SetOutline (Variables|Default|GetOutline) "None"))

(event EventPerformSelectedEnemyPawn
  (Class|OutlineComponent|SetOutline (Variables|Default|GetOutline) "Red"))

(fn ConstructionScript)

(fn MoveRule
  (params (InBoardStatus :type Array%20of%20Bytes))
  (Utilities|FlowControl|Sequence
    (:then_0
      (bind _aschinese_chess_board (Utilities|Casting|CastToChineseChessBoard (Class|BoardGameManager|GetBoard (Class|ChineseChessPawn|GetGameManagerPtr))))
      (LocalVariables|SetBoardPtr _aschinese_chess_board))
    (:then_1
      (LocalVariables|SetBoardSize (Class|ChineseChessBoard|GetBoardSize (LocalVariables|GetBoardPtr))))
    (:then_2
      (LocalVariables|SetCurrentSlotPos (Class|ChineseChessPawn|GetSlotPos))
      (bind _outpositions (|CallParentFunction InBoardStatus))
      (Utilities|FlowControl|Sequence
        (:then_0
          (Utilities|Array|Clear _outpositions))
        (:then_1
          (for _array_element (LocalVariables|GetDirections)
            (bind _output_get (LocalVariables|SetDetectionPos (+ _array_element (LocalVariables|GetCurrentSlotPos))))
            (bind _output_get_2 (LocalVariables|SetBlockDirection (+ (Math|Vector2D|MakeVector2D (Math|Conversions|ToFloat(Integer) (Math|Float|Truncate (.X (Math|Vector2D|BreakVector2D (/ _array_element 2.0))))) (Math|Conversions|ToFloat(Integer) (Math|Float|Truncate (.Y (Math|Vector2D|BreakVector2D (/ _array_element 2.0)))))) (LocalVariables|GetCurrentSlotPos))))
            (if (Class|ChineseChessBoard|CheckPositioninBoard (LocalVariables|GetBoardPtr) _output_get_2)
              (bind _returnvalue (Class|ChineseChessBoard|GetSlot (LocalVariables|GetBoardPtr) (LocalVariables|GetBlockDirection)))
              (if (not (Class|GameBaseBoardSlot|IsOccupied _returnvalue))
                (if (Class|ChineseChessBoard|CheckPositioninBoard (LocalVariables|GetBoardPtr) _output_get)
                  (bind _returnvalue_2 (Class|ChineseChessBoard|GetSlot (LocalVariables|GetBoardPtr) (LocalVariables|GetDetectionPos)))
                  (if (Class|GameBaseBoardSlot|IsOccupied _returnvalue_2)
                    (bind _aschinese_chess_pawn (Utilities|Casting|CastToChineseChessPawn (Class|GameBaseBoardSlot|GetOccupyingPawn _returnvalue_2)))
                    (if (not (Utilities|Enum|Equal(Enum) (Class|ChineseChessPawn|GetCamp _aschinese_chess_pawn) (Class|ChineseChessPawn|GetCamp)))
                      (Utilities|Array|AddUnique _outpositions (LocalVariables|GetDetectionPos)))
                    (else
                      (Utilities|Array|AddUnique _outpositions (LocalVariables|GetDetectionPos)))))))))
        (:then_2
          (return _outpositions))))))