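; Chinese chess Han-camp Cannon (Pao) pawn that supplies the piece's legal moves and selection outline.
; MoveRule clears the parent rule's result, then scans each direction, adding empty slots until a piece blocks the path.
; It then searches past that screen piece for the next occupied slot, adding it only if the occupant belongs to another camp.
; Selection events set the outline to blue for team, red for enemy, or none when idle.
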(event EventBeginPlay)

(event Collision|EventActorBeginOverlap
  (params (OtherActor :type Actor%20Object%20Reference)))

(event EventTick
  (params (DeltaSeconds :type Float%20%28single-precision%29)))

(event EventPerformSelectedTeamPawn
  (Class|OutlineComponent|SetOutline (Variables|Default|GetOutline) "Blue"))

(event EventPerformIdlePawn
  (Class|OutlineComponent|SetOutline (Variables|Default|GetOutline) "None"))

(event EventPerformSelectedEnemyPawn
  (Class|OutlineComponent|SetOutline (Variables|Default|GetOutline) "Red"))

(fn ConstructionScript)

(fn MoveRule
  (params (InBoardStatus :type Array%20of%20Bytes))
  (Utilities|FlowControl|Sequence
    (:then_0
      (bind _aschinese_chess_board (Utilities|Casting|CastToChineseChessBoard (Class|BoardGameManager|GetBoard (Class|ChineseChessPawn|GetGameManagerPtr))))
      (LocalVariables|SetBoardPtr _aschinese_chess_board))
    (:then_1
      (LocalVariables|SetBoardSize (Class|ChineseChessBoard|GetBoardSize (LocalVariables|GetBoardPtr))))
    (:then_2
      (LocalVariables|SetCurrentSlotPos (Class|ChineseChessPawn|GetSlotPos))
      (bind _outpositions (|CallParentFunction InBoardStatus))
      (Utilities|FlowControl|Sequence
        (:then_0
          (Utilities|Array|Clear _outpositions))
        (:then_1
          (for _array_element (LocalVariables|GetDirections)
            (while (LocalVariables|GetbContinueInteration)
              (bind _output_get (LocalVariables|SetDetectionPos (+ (Math|Conversions|ToVector2D(Vector) (* _array_element (LocalVariables|GetInterator))) (LocalVariables|GetCurrentSlotPos))))
              (if (Class|ChineseChessBoard|CheckPositioninBoard (LocalVariables|GetBoardPtr) _output_get)
                (bind _returnvalue (Class|ChineseChessBoard|GetSlot (LocalVariables|GetBoardPtr) (LocalVariables|GetDetectionPos)))
                (if (Class|GameBaseBoardSlot|IsOccupied _returnvalue)
                  (while (LocalVariables|GetbSearchAttackPos)
                    (bind _output_get_2 (LocalVariables|SetJumpPos (+ (Math|Conversions|ToVector2D(Vector) (* _array_element (LocalVariables|GetJumpInterator))) (LocalVariables|GetDetectionPos))))
                    (if (Class|ChineseChessBoard|CheckPositioninBoard (LocalVariables|GetBoardPtr) _output_get_2)
                      (bind _returnvalue_2 (Class|ChineseChessBoard|GetSlot (LocalVariables|GetBoardPtr) (LocalVariables|GetJumpPos)))
                      (if (Class|GameBaseBoardSlot|IsOccupied _returnvalue_2)
                        (bind _aschinese_chess_pawn (Utilities|Casting|CastToChineseChessPawn (Class|GameBaseBoardSlot|GetOccupyingPawn _returnvalue_2)))
                        (if (Utilities|Enum|Equal(Enum) (Class|ChineseChessPawn|GetCamp _aschinese_chess_pawn) (Class|ChineseChessPawn|GetCamp))
                          _
                          (else
                            (Utilities|Array|AddUnique _outpositions (LocalVariables|GetJumpPos))))
                        (LocalVariables|SetbContinueInteration false)
                        (LocalVariables|SetbSearchAttackPos false)
                        (else
                          (Math|Integer|IncrementInt (LocalVariables|GetJumpInterator))))
                      (else
                        (LocalVariables|SetbSearchAttackPos false)
                        (LocalVariables|SetbContinueInteration false))))
                  (else
                    (Utilities|Array|AddUnique _outpositions (LocalVariables|GetDetectionPos))
                    (Math|Integer|IncrementInt (LocalVariables|GetInterator))))
                (else
                  (LocalVariables|SetbContinueInteration false))))
            (LocalVariables|SetbContinueInteration true)
            (LocalVariables|SetbSearchAttackPos true)
            (LocalVariables|SetInterator 1)
            (LocalVariables|SetJumpInterator 1)))
        (:then_2
          (return _outpositions))))))