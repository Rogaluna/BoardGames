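; Han-side Shi (advisor) piece for Chinese chess, defining which board squares it can legally move to.
; MoveRule clears the parent rule's list, then tests each Directions offset from the current position against the palace area, shifted by team, and the board bounds.
; Empty squares and enemy-occupied squares are added to the returned moves.
; The idle and selection event hooks are empty.
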(event EventBeginPlay)

(event Collision|EventActorBeginOverlap
  (params (OtherActor :type Actor%20Object%20Reference)))

(event EventTick
  (params (DeltaSeconds :type Float%20%28single-precision%29)))

(event EventPerformSelectedTeamPawn)

(event EventPerformIdlePawn)

(event EventPerformSelectedEnemyPawn)

(fn ConstructionScript)

(fn MoveRule
  (params (InBoardStatus :type Array%20of%20Bytes) (PawnPos :type Vector%202D%20Structure%20%28by%20ref%29))
  (bind _output_get (LocalVariables|SetCurrentSlotPos PawnPos))
  (bind _outpositions (|CallParentFunction InBoardStatus _output_get))
  (Utilities|FlowControl|Sequence
    (:then_0
      (Utilities|Array|Clear _outpositions))
    (:then_1
      (for _array_element (LocalVariables|GetDirections)
        (bind _output_get_2 (LocalVariables|SetDetectionPos (+ _array_element (LocalVariables|GetCurrentSlotPos))))
        (if (and (Math|Float|InRange(Float) (.X (Math|Vector2D|BreakVector2D (- _output_get_2 (Utilities|Select :Index (Class|ChineseChessSetFunctionLibrary|IsBelongto (Class|ChineseChessSetFunctionLibrary|Encode (Class|ChineseChessPawn|GetPawnType))) :Chu "" :Han "(X=0.000000,Y=7.000000)")))) 3.0 5.0) (Math|Float|InRange(Float) (.Y (Math|Vector2D|BreakVector2D (- _output_get_2 (Utilities|Select :Index (Class|ChineseChessSetFunctionLibrary|IsBelongto (Class|ChineseChessSetFunctionLibrary|Encode (Class|ChineseChessPawn|GetPawnType))) :Chu "" :Han "(X=0.000000,Y=7.000000)")))) 0.0 2.0))
          (if (Class|ChineseChessSetFunctionLibrary|CheckPositioninBoard _output_get_2)
            (if (!= (Utilities|Array|Get(acopy) InBoardStatus (Class|ChineseChessSetFunctionLibrary|TransformPostoIndex (LocalVariables|GetDetectionPos))) 0)
              (if (not (Utilities|Enum|Equal(Enum) (Class|ChineseChessSetFunctionLibrary|IsBelongto (Utilities|Array|Get(acopy) InBoardStatus (Class|ChineseChessSetFunctionLibrary|TransformPostoIndex (LocalVariables|GetDetectionPos)))) (Class|ChineseChessSetFunctionLibrary|IsBelongto (Class|ChineseChessSetFunctionLibrary|Encode (Class|ChineseChessPawn|GetPawnType)))))
                (Utilities|Array|AddUnique _outpositions (LocalVariables|GetDetectionPos)))
              (else
                (Utilities|Array|AddUnique _outpositions (LocalVariables|GetDetectionPos))))))))
    (:then_2
      (return _outpositions))))